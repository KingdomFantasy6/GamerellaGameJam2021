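; Player character with mouse look, axis-driven movement, a pause menu and an energy pool.
; Mouse X yaws the controller and movement follows the actor's axes, while mouse Y pitches the SpringArm, then clamps it to a zero-width range.
; Pause toggles game pause and UI_PauseMenu, but the first press only creates the widget.
; ReduceEnergy subtracts energy and reloads the current level at zero or below.
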(event `InputAxisKey|MouseX`
  (params (AxisValue :type "Float (single-precision)"))
  ;[1 1 1] use mouse to turn camera and player
  (`self.AddControllerYawInput` AxisValue))

(event `InputAxisKey|MouseY`
  (params (AxisValue :type "Float (single-precision)"))
  ;[1 1 1] use mouse to turn camera and player
  (`SceneComponent.K2_AddLocalRotation` (`self.SpringArm`) (`KismetMathLibrary.MakeRotator` 0.0 AxisValue) false false)
  (`SceneComponent.K2_SetRelativeRotation` (`self.SpringArm`) (`KismetMathLibrary.MakeRotator` 0.0 (`KismetMathLibrary.ClampAngle` (.pitch (`SpringArmComponent.GetTargetRotation` (`self.SpringArm`))))) false false))

(event `InputAxis|Move_ForwardBack`
  (params (AxisValue :type "Float (single-precision)"))
  ;[1 1 1] movement
  (`self.AddMovementInput` (`self.GetActorForwardVector`) AxisValue))

(event `InputAxis|Move_leftRight`
  (params (AxisValue :type "Float (single-precision)"))
  ;[1 1 1] movement
  (`self.AddMovementInput` (`self.GetActorRightVector`) AxisValue))

(event `InputAction|Pause`
  (params (Key :type "Key Structure"))
  (bind _returnvalue (`GameplayStatics.GetPlayerController` 0))
  (bind _pausemenuref (`self.PauseMenuRef`))
  ;[1 1 1] Pause Menu
  (:`Pressed`
    (`/Engine/EditorBlueprintResources/StandardMacros.IsValid` (`self.PauseMenuRef`)
      (:`Is Valid`
        (if (`GameplayStatics.IsGamePaused`)
          (`Widget.RemoveFromParent` _pausemenuref)
          (`GameplayStatics.SetGamePaused` false)
          (set `PlayerController.bShowMouseCursor` false _returnvalue)
          (`WidgetBlueprintLibrary.SetInputMode_GameOnly` _returnvalue)
          (else
            (`UserWidget.AddToViewport` _pausemenuref 0)
            (`GameplayStatics.SetGamePaused` true)
            (set `PlayerController.bShowMouseCursor` false _returnvalue)
            (`WidgetBlueprintLibrary.SetInputMode_GameAndUIEx` _returnvalue _pausemenuref))))
      (:`Is Not Valid`
        (bind _returnvalue_2 (`|CreateWidget` "/Game/UI_Widgets/UI_PauseMenu.UI_PauseMenu_C"))
        (set `self.PauseMenuRef` _returnvalue_2)))))

(fn `ReduceEnergy`
  (params (EnergyLost :type Integer))
  (bind _output_get (set `self.CurrentEnergy` (- (`self.CurrentEnergy`) EnergyLost)))
  (if (<= _output_get 0)
    (bind _returnvalue (`GameplayStatics.GetCurrentLevelName` true))
    (`GameplayStatics.OpenLevel` (`KismetStringLibrary.Conv_StringToName` _returnvalue))))

(fn `UserConstructionScript`)