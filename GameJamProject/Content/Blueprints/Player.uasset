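; Player Blueprint that handles grid-like step movement and the pause menu.
; Each directional input press shifts a TargetPosition variable by a fixed step along X or Y; nothing in this graph applies it to the actor.
; The Pause input lazily creates and caches UI_PauseMenu, then toggles game pause, the menu, mouse cursor visibility and input mode.
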(event `InputAction|MoveUp`
  (params (Key :type "Key Structure"))
  ;[1 1 1] BASIC player movement
  (:`Pressed`
    (set `self.TargetPosition` (+ (`self.TargetPosition`) (100.0 0.0 0.0)))))

(event `InputAction|Pause` :paused true
  (params (Key :type "Key Structure"))
  (bind _returnvalue (`GameplayStatics.GetPlayerController` 0))
  (bind _pausemenuref (`self.PauseMenuRef`))
  ;[1 1 1] Pause Functionality
  (:`Pressed`
    (`/Engine/EditorBlueprintResources/StandardMacros.IsValid` (`self.PauseMenuRef`)
      (:`Is Valid`
        _)
      (:`Is Not Valid`
        (bind _returnvalue_2 (`|CreateWidget` "/Game/UI_Widgets/UI_PauseMenu.UI_PauseMenu_C"))
        (set `self.PauseMenuRef` _returnvalue_2)))
    (if (`GameplayStatics.IsGamePaused`)
      (`Widget.RemoveFromParent` _pausemenuref)
      (`GameplayStatics.SetGamePaused` false)
      (set `PlayerController.bShowMouseCursor` false _returnvalue)
      (`WidgetBlueprintLibrary.SetInputMode_GameOnly` _returnvalue)
      (else
        (`UserWidget.AddToViewport` _pausemenuref 0)
        (`GameplayStatics.SetGamePaused` true)
        (set `PlayerController.bShowMouseCursor` true _returnvalue)
        (`WidgetBlueprintLibrary.SetInputMode_GameAndUIEx` _returnvalue _pausemenuref)))))

(event `InputAction|MoveDown`
  (params (Key :type "Key Structure"))
  ;[1 1 1] BASIC player movement
  (:`Pressed`
    (set `self.TargetPosition` (+ (`self.TargetPosition`) (-100.0 0.0 0.0)))))

(event `InputAction|MoveRight`
  (params (Key :type "Key Structure"))
  ;[1 1 1] BASIC player movement
  (:`Pressed`
    (set `self.TargetPosition` (+ (`self.TargetPosition`) (0.0 100.0 0.0)))))

(event `InputAction|MoveLeft`
  (params (Key :type "Key Structure"))
  ;[1 1 1] BASIC player movement
  (:`Pressed`
    (set `self.TargetPosition` (+ (`self.TargetPosition`) (0.0 -100.0 0.0)))))

(fn `UserConstructionScript`)